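; BP_PlayerBase is a player base Blueprint that moves a physics-driven static mesh with camera-relative input.
; MoveForward and MoveRight pass the camera's forward or right vector through GetMovementDirection, which scales it by axis value and MoveSpeed.
; The resulting X and Y drive AddForce as acceleration, while each axis event replaces Z with a downward force proportional to current speed.
; Turn and LookUp feed controller yaw and pitch.
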(event EventBeginPlay)

(event Collision|EventActorBeginOverlap
  (params (OtherActor :type Actor%20Object%20Reference)))

(event EventTick
  (params (DeltaSeconds :type Float%20%28single-precision%29)))

(event Input|AxisEvents|InputAxisMoveForward
  (params (AxisValue :type Float%20%28single-precision%29))
  (bind _returnvalue (Input|AxisValues|GetMoveForward))
  (bind _camera (Variables|Default|GetCamera))
  (bind _returnvalue_2 (Math|Vector|GetForwardVector _camera))
  (bind _movementresult (CallFunction|GetMovementDirection _returnvalue_2 _returnvalue))
  (Physics|AddForce (Variables|Default|GetStaticMesh) (Math|Vector|MakeVector (.x _movementresult) (.y _movementresult) (* (Math|Vector|VectorLength (Transformation|GetVelocity)) -0.45)) "None" true))

(event Input|AxisEvents|InputAxisMoveRight
  (params (AxisValue :type Float%20%28single-precision%29))
  (bind _returnvalue (Input|AxisValues|GetMoveRight))
  (bind _camera (Variables|Default|GetCamera))
  (bind _returnvalue_2 (Math|Vector|GetRightVector _camera))
  (bind _movementresult (CallFunction|GetMovementDirection _returnvalue_2 _returnvalue))
  (Physics|AddForce (Variables|Default|GetStaticMesh) (Math|Vector|MakeVector (.x _movementresult) (.y _movementresult) (* (Math|Vector|VectorLength (Transformation|GetVelocity)) -0.45)) "None" true))

(event Input|AxisEvents|InputAxisLookUp
  (params (AxisValue :type Float%20%28single-precision%29))
  (Pawn|Input|AddControllerPitchInput AxisValue))

(event Input|AxisEvents|InputAxisTurn
  (params (AxisValue :type Float%20%28single-precision%29))
  (Pawn|Input|AddControllerYawInput AxisValue))

(fn ConstructionScript)

(fn GetMovementDirection
  (params (InputDirection :type Vector) (MoveInputAxis :type Float%20%28single-precision%29))
  (return (* (* InputDirection MoveInputAxis) (Variables|Default|GetMoveSpeed))))