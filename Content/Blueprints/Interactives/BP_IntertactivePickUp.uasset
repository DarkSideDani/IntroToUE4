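; Interactive pickup that is magnetically drawn to the player and destroys itself when interacted with.
; When a BP_PlayerBase overlaps the magnetic radius collider, it stores the player and its own start location, then plays a sped-up timeline.
; Each timeline update lerps the pickup from that start toward the player's current location, so it tracks a moving target.
; Interact runs the parent logic, then destroys the actor.
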(event OnComponentBeginOverlap(MagneticRadiusCollider)
  (params (OverlappedComponent :type Primitive%20Component%20Object%20Reference) (OtherActor :type Actor%20Object%20Reference) (OtherComp :type Primitive%20Component%20Object%20Reference) (OtherBodyIndex :type Integer) (bFromSweep :type Boolean) (SweepResult :type Hit%20Result%20Structure%20%28by%20ref%29))
  (bind _asbp_player_base (Utilities|Casting|CastToBP_PlayerBase OtherActor))
  (Variables|Default|SetPlayer%20Ref _asbp_player_base)
  (Variables|Default|SetStartLocation (Transformation|GetActorLocation))
  (bind _movespeed (Timeline|MoveToPlayerTimeline PlayFromStart)
    (:Update
      (Transformation|SetActorLocation (Math|Vector|Lerp(Vector) (Variables|Default|GetStartLocation) (Transformation|GetActorLocation (Variables|Default|GetPlayer%20Ref)) _movespeed) false false))))

(event EventBeginPlay
  (Components|Timeline|SetPlayRate (Variables|Default|GetMoveToPlayerTimeline) 2.5))

(fn ConstructionScript
  (|CallParentFunction))

(fn Interact
  (params (OverlappedActor :type Actor%20Object%20Reference))
  (|CallParentFunction OverlappedActor)
  (Actor|DestroyActor))