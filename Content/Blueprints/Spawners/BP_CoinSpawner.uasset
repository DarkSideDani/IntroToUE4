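; BP_CoinSpawner lays out coin pickups at even Spacing intervals along a spline.
; The construction script previews them with static mesh components stored in CoinMeshArray.
; On BeginPlay it destroys those meshes and spawns BP_IntertactivePickUp actors at the same distances.
; Both passes share ReturnSplineLocationAndRotation, which returns spline-local transforms, so SpawnActor receives local rather than world coordinates.
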(event EventBeginPlay
  (bind (_location _rotation) (CallFunction|ReturnSplineLocationandRotation))
  (for _array_element (Variables|Default|GetCoinMeshArray)
    (Components|DestroyComponent _array_element))
  (for _index (range 0 (Math|Float|Truncate (/ (Spline|GetSplineLength (Variables|Default|GetSpline)) (Variables|Default|GetSpacing))))
    (Variables|Default|SetSplinePoint _index)
    (Game|SpawnActorfromClass "/Game/Blueprints/Interactives/BP_IntertactivePickUp.BP_IntertactivePickUp_C" (Math|Transform|MakeTransform _location _rotation "1,1,1") "Undefined" 0 0)))

(fn ConstructionScript
  (bind (_location _rotation) (CallFunction|ReturnSplineLocationandRotation))
  (Utilities|Array|Clear (Variables|Default|GetCoinMeshArray))
  (for _index (range 0 (Math|Float|Truncate (/ (Spline|GetSplineLength (Variables|Default|GetSpline)) (Variables|Default|GetSpacing))))
    (Variables|Default|SetSplinePoint _index)
    (bind _returnvalue (AddComponent|AddStaticMeshComponent false (Math|Transform|MakeTransform _location _rotation "1,1,1")))
    (Utilities|Array|Add (Variables|Default|GetCoinMeshArray) _returnvalue)))

(fn ReturnSplineLocationandRotation
  (bind _spline (Variables|Default|GetSpline))
  (bind _spacing (Variables|Default|GetSpacing))
  (bind _splinepoint (Variables|Default|GetSplinePoint))
  (bind _returnvalue (* _splinepoint _spacing))
  (return (Spline|GetLocationatDistanceAlongSpline _spline _returnvalue "Local") (Spline|GetRotationatDistanceAlongSpline _spline _returnvalue "Local")))