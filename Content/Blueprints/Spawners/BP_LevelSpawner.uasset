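; BP_LevelSpawner is a spline-driven actor that builds level floor geometry along an editable path.
; Its construction script divides the spline length by SectionLength and adds a collision-enabled spline mesh for each section, using distinct start, straight and end floor meshes.
; ReturnSplinePositionAndTangent supplies each section's local-space endpoints and tangents, sampled by distance along the spline so the meshes bend with it.
; The event graph contains no active logic.
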(event EventBeginPlay)

(event Collision|EventActorBeginOverlap
  (params (OtherActor :type Actor%20Object%20Reference)))

(event EventTick
  (params (DeltaSeconds :type Float%20%28single-precision%29)))

(fn ConstructionScript
  (bind (_startpos _starttangent _endpos _endtangent) (CallFunction|ReturnSplinePositionandTangent))
  (for _index (range 0 (Math|Float|Truncate (/ (Spline|GetSplineLength (Variables|Default|GetSpline)) (Variables|Default|GetSectionLength))))
    (Variables|Default|SetSplinePoint _index)
    (bind _returnvalue (AddComponent|AddSplineMeshComponent false))
    (Components|StaticMesh|SetStaticMesh _returnvalue (select (== (Variables|Default|GetSplinePoint) 0) "/Game/Assets/Meshes/SM_FloorStart.SM_FloorStart" (select (== (Variables|Default|GetSplinePoint) (Math|Float|Truncate (/ (Spline|GetSplineLength (Variables|Default|GetSpline)) (Variables|Default|GetSectionLength)))) "/Game/Assets/Meshes/SM_FloorEnd.SM_FloorEnd" "/Game/Assets/Meshes/SM_FloorStraight.SM_FloorStraight")))
    (Collision|SetCollisionEnabled _returnvalue "QueryAndPhysics")
    (SplineMesh|SetStartandEnd _returnvalue _startpos _starttangent _endpos _endtangent true :!class /Script/Engine.SplineMeshComponent)))

(fn ReturnSplinePositionandTangent
  (bind _spline (Variables|Default|GetSpline))
  (bind _sectionlength (Variables|Default|GetSectionLength))
  (bind _splinepoint (Variables|Default|GetSplinePoint))
  (bind _spline_2 (Variables|Default|GetSpline))
  (bind _sectionlength_2 (Variables|Default|GetSectionLength))
  (bind _splinepoint_2 (Variables|Default|GetSplinePoint))
  (bind _returnvalue (* _splinepoint_2 _sectionlength_2))
  (bind _returnvalue_2 (+ _splinepoint 1))
  (bind _returnvalue_3 (* _returnvalue_2 _sectionlength))
  (return (Spline|GetLocationatDistanceAlongSpline _spline_2 _returnvalue "Local") (Spline|GetTangentatDistanceAlongSpline _spline_2 _returnvalue "Local") (Spline|GetLocationatDistanceAlongSpline _spline _returnvalue_3 "Local") (Spline|GetTangentatDistanceAlongSpline _spline _returnvalue_3 "Local")))